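; Door actor that slides upward when the ThirdPersonCharacter overlaps it holding at least the required number of keys, and lowers when they leave.
; BeginPlay caches the start location and a raised target offset by Elevation.
; Overlap events set an Open flag, and Tick lerps the actor toward the matching position by DeltaSeconds times Speed, giving an eased motion.
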(event EventBeginPlay
  (bind _returnvalue (Transformation|GetActorLocation))
  (Variables|Default|SetInitialPos (Transformation|GetActorLocation))
  (Variables|Default|SetUpPos (Math|Vector|MakeVector (.x _returnvalue) (.y _returnvalue) (+ (.z _returnvalue) (Variables|Default|GetElevation)))))

(event Collision|EventActorBeginOverlap
  (params (OtherActor :type Actor%20Object%20Reference))
  (if (== (Utilities|GetClass OtherActor) "/Game/ThirdPersonBP/Blueprints/ThirdPersonCharacter.ThirdPersonCharacter_C")
    (bind _asthird_person_character (Utilities|Casting|CastToThirdPersonCharacter OtherActor))
    (if (>= (Variables|/Game/ThirdPersonBP/Blueprints/ThirdPersonCharacter.ThirdPersonCharacter_C|GetKeys _asthird_person_character) (Variables|Default|GetKeysNeeded))
      (Variables|Default|SetOpen true))))

(event EventTick
  (params (DeltaSeconds :type Float%20%28single-precision%29))
  (if (Variables|Default|GetOpen)
    (Transformation|SetActorLocation (Math|Vector|Lerp(Vector) (Transformation|GetActorLocation) (Variables|Default|GetUpPos) (* DeltaSeconds (Variables|Default|GetSpeed))) false false)
    (else
      (Transformation|SetActorLocation (Math|Vector|Lerp(Vector) (Transformation|GetActorLocation) (Variables|Default|GetInitialPos) (* DeltaSeconds (Variables|Default|GetSpeed))) false false))))

(event Collision|EventActorEndOverlap
  (params (OtherActor :type Actor%20Object%20Reference))
  (if (== (Utilities|GetClass OtherActor) "/Game/ThirdPersonBP/Blueprints/ThirdPersonCharacter.ThirdPersonCharacter_C")
    (Variables|Default|SetOpen false)))

(fn ConstructionScript)