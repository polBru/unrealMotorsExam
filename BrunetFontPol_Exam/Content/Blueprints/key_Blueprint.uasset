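; Key pickup actor that the third-person character collects by overlapping it.
; On overlap it plays one of two key sounds at its mesh location, chosen at random with randomized volume and pitch.
; It then increments the character's Keys count and destroys itself.
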(event Collision|EventActorBeginOverlap
  (params (OtherActor :type Actor%20Object%20Reference))
  (bind _returnvalue (Math|Random|RandomFloatinRange 0.7 1.2))
  (bind _returnvalue_2 (Math|Random|RandomFloatinRange 0.7 1.2))
  (if (== (Utilities|GetClass OtherActor) "/Game/ThirdPersonBP/Blueprints/ThirdPersonCharacter.ThirdPersonCharacter_C")
    (if (== (Math|Random|RandomIntegerinRange 0 1) 0)
      (Audio|PlaySoundatLocation "/Game/Audio/Key.Key" (Transformation|GetWorldLocation (Variables|Debug|GetStaticMeshComponent)) "0, 0, 0" (* _returnvalue 2.5) _returnvalue 0.0 0 0 0)
      (else
        (Audio|PlaySoundatLocation "/Game/Audio/Key2.Key2" (Transformation|GetWorldLocation (Variables|Debug|GetStaticMeshComponent)) "0, 0, 0" (* _returnvalue_2 2.5) _returnvalue_2 0.0 0 0 0)))
    (bind _asthird_person_character (Utilities|Casting|CastToThirdPersonCharacter OtherActor))
    (Variables|/Game/ThirdPersonBP/Blueprints/ThirdPersonCharacter.ThirdPersonCharacter_C|SetKeys _asthird_person_character (+ (Variables|/Game/ThirdPersonBP/Blueprints/ThirdPersonCharacter.ThirdPersonCharacter_C|GetKeys _asthird_person_character) 1))
    (Actor|DestroyActor)))

(fn ConstructionScript)